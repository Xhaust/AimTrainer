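; First-person player Blueprint that handles looking and hitscan shooting, using an aim trainer input mapping.
; BeginPlay adds the Enhanced Input mapping context, and the look action drives controller yaw and pitch.
; Shooting line-traces forward from the camera on the Camera channel with debug drawing, then applies damage to the hit actor.
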(event Input|EnhancedActionEvents|EnhancedInputActionIA_Shoot
  (params (ActionValue :type Boolean) (ElapsedSeconds :type Float%20%28double-precision%29) (TriggeredSeconds :type Float%20%28double-precision%29) (InputAction :type Input%20Action%20Object%20Reference :default "/Game/IA_Shoot.IA_Shoot"))
  (bind _desiredview (Class|CameraComponent|GetCameraView (Variables|Default|GetFirstPersonCamera) 0.0))
  (bind _outhit (Collision|LineTraceByChannel (.Location (Utilities|Struct|BreakMinimalViewInfo _desiredview)) (+ (.Location (Utilities|Struct|BreakMinimalViewInfo _desiredview)) (* (Math|Rotator|GetRotationXVector (.Rotation (Utilities|Struct|BreakMinimalViewInfo _desiredview))) (Math|Conversions|ToVector(Float) 1.5e+03))) "TraceTypeQuery2" false 0 "ForDuration" true "(R=1.000000,G=0.000000,B=0.000000,A=1.000000)" "(R=0.000000,G=1.000000,B=0.000000,A=1.000000)" 1e+01))
  (Game|Damage|ApplyDamage (.HitActor (Collision|BreakHitResult _outhit)) 1.0 0 0))

(event Input|EnhancedActionEvents|EnhancedInputActionIA_Look
  (params (ActionValue :type Vector%202D%20Structure) (ElapsedSeconds :type Float%20%28double-precision%29) (TriggeredSeconds :type Float%20%28double-precision%29) (InputAction :type Input%20Action%20Object%20Reference :default "/Game/IA_Look.IA_Look"))
  (bind (_x _y) (Math|Vector2D|BreakVector2D ActionValue))
  (Pawn|Input|AddControllerYawInput _x)
  (Pawn|Input|AddControllerPitchInput _y))

(event EventBeginPlay
  (bind _asplayer_controller (Utilities|Casting|CastToPlayerController (Pawn|GetController)))
  (Input|AddMappingContext (PlayerController|LocalPlayerSubsystems|GetEnhancedInputLocalPlayerSubsystem _asplayer_controller) "/Game/IMC_AimTrainer.IMC_AimTrainer" 0 "(bIgnoreAllPressedKeysUntilRelease=True,bForceImmediately=False,bNotifyUserSettings=False)"))

(event Collision|EventActorBeginOverlap
  (params (OtherActor :type Actor%20Object%20Reference)))

(event EventTick
  (params (DeltaSeconds :type Float%20%28single-precision%29)))

(fn ConstructionScript)